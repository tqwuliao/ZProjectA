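; Global helper function library that gives access to the game mode and handles coordinate math for a three-column grid of target positions.
; GetMyGameMode returns the current game mode cast to NewGameMode.
; Index helpers convert between column/row and a flat row-major index.
; GetTargetPosition maps grid cells to locations at fixed height through linear math expressions, with grid Y driving world X and grid X driving world Y.
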(fn GetMyGameMode
  (bind _asnew_game_mode (Utilities|Casting|CastToNewGameMode (Game|GetGameMode (LocalVariables|Get__WorldContext))))
  (return _asnew_game_mode))

(fn GetTargetPosition
  (params (X :type Integer) (Y :type Integer))
  (return (Math|Vector|MakeVector (|((a*28)-208) (Math|Conversions|ToFloat(Integer) Y)) (|(28-(a*28)) (Math|Conversions|ToFloat(Integer) X)) 1.1e+02)))

(fn GetIndexfromXY
  (params (X :type Integer) (Y :type Integer))
  (return (+ X (* Y 3))))

(fn GetXYfromIndex
  (params (Index :type Integer))
  (return (Math|Integer|%(Integer) Index 3) (/ Index 3)))