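; MarkInst is a board mark actor for a 3x3 grid game, registering itself with the game mode on BeginPlay.
; GetXY converts its Index to a column and row, and MarkValue returns a constant 1.
; Win swaps the decal to a dynamic material instance and sets its highlight offset time to one second after the current game time.
; Fet, overlap and tick are empty.
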(event `self.ReceiveBeginPlay`
  (`/Game/Blueprints/NewGameMode.RegistMark` (`/Game/Blueprints/GlobalFunctions.GetMyGameMode`) self))

(fn `Fet`)

(fn `GetXY`
  (returns (X :type Integer) (Y :type Integer))
  (bind _index (`self.Index`))
  (return (mod _index 3) (/ _index 3)))

(fn `MarkValue`
  (returns (Value :type Integer))
  (return 1))

(fn `UserConstructionScript`)

(fn `Win`
  (bind _decal (`self.Decal`))
  (bind _returnvalue (`KismetMaterialLibrary.CreateDynamicMaterialInstance` (`DecalComponent.DecalMaterial` _decal)))
  (`MaterialInstanceDynamic.SetScalarParameterValue` _returnvalue "HighlightOffsetTime" (+ (`KismetSystemLibrary.GetGameTimeInSeconds`) 1.0))
  (`DecalComponent.SetDecalMaterial` _decal _returnvalue))