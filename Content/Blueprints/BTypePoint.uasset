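; BTypePoint is the AI-driven enemy variant of a parent point class, using the enemy mark class.
; On BeginPlay it loads level 0 settings from the AISettingPerLevel data table, with levels clamped to 0–5.
; BeginCalculate changes the current state and runs the BasicEnemyLogic behavior tree through its AI controller.
; Apply changes state, forwards X/Y to the parent and calls OnPlayerBeginApply.
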(event `self.ReceiveBeginPlay`
  (`parent.ReceiveBeginPlay`)
  (`self.SetAILevel` 0))

(event `self.Apply`
  (params (TargetPosition :type "Vector Structure") (X :type Integer) (Y :type Integer))
  (set `self.CurrentState` "NewEnumerator2")
  (`parent.Apply` (0.0 0.0 0.0) X Y)
  (`self.OnPlayerBeginApply`))

(fn `BeginCalculate`
  (set `self.CurrentState` "NewEnumerator1")
  (`AIController.RunBehaviorTree` (`AIBlueprintHelperLibrary.GetAIController` self) "/Game/AI/BasicEnemyLogic.BasicEnemyLogic"))

(fn `FetchMarkClz`
  (returns (Clz :type "/Game/Blueprints/MarkInst Class Reference"))
  (return "/Game/Blueprints/MarkInst_Enemy.MarkInst_Enemy_C"))

(fn `SetAILevel`
  (params (Level :type Integer))
  (`KismetSystemLibrary.PrintText` (`|FormatText` "设置AI级别 {0}" Level))
  (bind _returnvalue (`|GetDataTableRow` "/Game/Blueprints/Data/AISettingPerLevel.AISettingPerLevel" (`KismetStringLibrary.Conv_StringToName` (`KismetStringLibrary.Conv_IntToString` (`KismetMathLibrary.Clamp` Level 0 5))))
    (:`then`
      (set `self.AISetting` _returnvalue))))

(fn `UserConstructionScript`)