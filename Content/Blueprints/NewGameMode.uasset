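; Tic-tac-toe game mode that tracks placed marks on a 3x3 board and decides when a round ends.
; RegistMark stores each mark, then either broadcasts the winner (0 for a draw) and highlights the winning line, or signals the owner's turn finished.
; CheckIfPointWinning tests only lines through the newest mark using modulo and mirrored coordinates.
; ClearAllMarks destroys marks to reset the board; ShowPointWinning is an unfinished stub.
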(event `self.ReceiveBeginPlay`
  (`KismetArrayLibrary.Array_Resize` (`self.CurrentMarks`) 9))

(fn `CheckIfPointWinning`
  (params (X :type Integer) (Y :type Integer) (Type :type Integer))
  (returns (ReturnValue :type Boolean) (Index :type "Array of Integer"))
  (bind (_type _index) (`self.HasMarkOnIndex` 0))
  (bind (_type_2 _index_2) (`self.HasMarkOnIndex` 1 1))
  (bind (_type_3 _index_3) (`self.HasMarkOnIndex` 2))
  (bind (_type_4 _index_4) (`self.HasMarkOnIndex` 0 2))
  (bind (_type_5 _index_5) (`self.HasMarkOnIndex` 2 2))
  (bind _index_6 (`/Game/Blueprints/GlobalFunctions.GetIndexFromXY` X Y))
  (bind _type_6 (`local.Type`))
  (bind _type_7 (`local.Type`))
  (bind _type_8 (`local.Type`))
  (bind _y (`local.Y`))
  (bind _x (`local.X`))
  (bind _type_9 (`local.Type`))
  (bind _type_10 (`local.Type`))
  (bind _y_2 (`local.Y`))
  (bind _x_2 (`local.X`))
  (bind (_type_11 _index_7) (`self.HasMarkOnIndex` (- 2 _x) (- 2 _y)))
  (bind (_type_12 _index_8) (`self.HasMarkOnIndex` (mod (+ X 2) 3) Y))
  (bind (_type_13 _index_9) (`self.HasMarkOnIndex` (mod (+ X 1) 3) Y))
  (bind _returnvalue (and (== (`local.X`) 1) (== (`local.Y`) 1)))
  (bind (_type_14 _index_10) (`self.HasMarkOnIndex` _x_2 (mod (+ _y_2 2) 3)))
  (bind (_type_15 _index_11) (`self.HasMarkOnIndex` _x_2 (mod (+ _y_2 1) 3)))
  (bind _returnvalue_2 (and (== _type _type_6) _returnvalue (== _type_6 _type_5)))
  (bind _returnvalue_3 (and (== _type_3 _type_8) _returnvalue (== _type_8 _type_4)))
  (bind _returnvalue_4 (and (== _type_11 _type_10) (== _type_10 _type_2) (or (!= _x 1) (!= _y 1))))
  (bind _returnvalue_5 (and (== _type_14 _type_9) (== _type_9 _type_15)))
  (return (or (and (== _type_12 _type_7) (== _type_7 _type_13)) _returnvalue_5 _returnvalue_4 _returnvalue_3 _returnvalue_2) (select `bool` (or _returnvalue_3 _returnvalue_2) :`false` (select `bool` _returnvalue_4 :`false` (select `bool` _returnvalue_5 :`false` (`|MakeArray` _index_8 _index_9 _index_6) :`true` (`|MakeArray` _index_6 _index_10 _index_11)) :`true` (`|MakeArray` _index_7 _index_2 (`/Game/Blueprints/GlobalFunctions.GetIndexFromXY` _x _y))) :`true` (select `bool` _returnvalue_3 :`false` (`|MakeArray` _index _index_5 4) :`true` (`|MakeArray` _index_3 _index_4 4)))))

(fn `ClearAllMarks`
  (for _array_element (`self.CurrentMarks`)
    (`/Engine/EditorBlueprintResources/StandardMacros.IsValid` _array_element
      (:`Is Valid`
        (`self.K2_DestroyActor` _array_element))))
  (set `self.CurrentMarks` (`|MakeArray` null null null null null null null null null :!type "/Game/Blueprints/MarkInst Object Reference")))

(fn `EmptyNodeList`
  (returns (List :type "Array of Integer"))
  (locals (NewLocalVar_0 :type "Array of Integer"))
  (for _index (range 9)
    (`/Engine/EditorBlueprintResources/StandardMacros.IsValid` (`|GetArrayItem` (`self.CurrentMarks`) _index)
      (:`Is Not Valid`
        (`KismetArrayLibrary.Array_Add` (`local.NewLocalVar_0`) _index))))
  (return (`local.NewLocalVar_0`)))

(fn `HasMarkOnIndex`
  (params (X :type Integer) (Y :type Integer))
  (returns (Type :type Integer) (Index :type Integer))
  (bind _returnvalue (+ X (* Y 3)))
  (bind _output (`|GetArrayItem` (`self.CurrentMarks`) _returnvalue))
  (if (`KismetSystemLibrary.IsValid` _output)
    (return (`/Game/Blueprints/MarkInst.MarkValue` _output) _returnvalue)
    (else
      (return 0 _returnvalue))))

(fn `RegistMark`
  (params (Inst :type "/Game/Blueprints/MarkInst Object Reference"))
  (bind _value (`/Game/Blueprints/MarkInst.MarkValue` Inst))
  (bind _index (`/Game/Blueprints/MarkInst.Index` Inst))
  (bind (_x _y) (`/Game/Blueprints/GlobalFunctions.GetXYFromIndex` _index))
  (bind (_returnvalue _index_2) (`self.CheckIfPointWinning` _x _y _value))
  (bind _returnvalue_2 (`KismetMathLibrary.SelectInt` _value 0 _returnvalue))
  (`KismetArrayLibrary.Array_Set` (`self.CurrentMarks`) _index Inst)
  (if (or _returnvalue (`KismetArrayLibrary.Array_IsEmpty` (`self.EmptyNodeList`)))
    (`self.OnRoundFinished` _returnvalue_2)
    (if (> _returnvalue_2 0)
      (for _array_element _index_2
        (`/Game/Blueprints/MarkInst.Win` (`|GetArrayItem` (`self.CurrentMarks`) _array_element))))
    (else
      (bind _asatype_point (cast `/Game/Blueprints/ATypePoint` (`self.GetOwner` Inst)))
      (`/Game/Blueprints/ATypePoint.OnPlayerTurnFinished` _asatype_point))))

(fn `ShowPointWinning`
  (params (X :type Integer) (Y :type Integer) (Type :type Integer))
  (bind _type (`local.Type`))
  (`|ExecutionSequence`
    (:`then_0`
      (if (and (== (`self.HasMarkOnIndex` (mod (+ X 2) 3) Y) _type) (== _type (`self.HasMarkOnIndex` (mod (+ X 1) 3) Y)))
        (return)))))

(fn `UserConstructionScript`)