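; Movable pointer actor that travels over a grid and places a mark on the chosen X/Y cell.
; SetTargetPoint either snaps it, stamping game time into the mesh's custom primitive data, or glides it via InterpToMovement when the target shifts enough.
; Apply glides it to the cell, plays a timeline-driven vertical drop after a short delay, then spawns the MarkInst class there with the cell's index.
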(event `Apply`
  (params (TargetPosition :type "Vector Structure") (X :type Integer) (Y :type Integer))
  (bind _location (`/Game/Blueprints/GlobalFunctions.GetTargetPosition` X Y))
  (bind _interptomovement (`self.InterpToMovement`))
  (set `InterpToMovementComponent.Duration` 0.2 _interptomovement)
  (`InterpToMovementComponent.ResetControlPoints` _interptomovement)
  (`InterpToMovementComponent.AddControlPointPosition` _interptomovement (`self.K2_GetActorLocation`) false)
  (`InterpToMovementComponent.AddControlPointPosition` _interptomovement _location false)
  (`InterpToMovementComponent.FinaliseControlPoints` _interptomovement)
  (`InterpToMovementComponent.RestartMovement` _interptomovement 1.0)
  (`KismetSystemLibrary.Delay` 0.2)
  (bind (_direction _newtrack_0) (`Timeline|TimeDrop` :!via `PlayFromStart`)
    (:`Update`
      (`self.K2_SetActorLocation` (+ _location (`KismetMathLibrary.MakeVector` 0.0 0.0 _newtrack_0))))
    (:`Finished`
      (`|SpawnActorFromClass` (`self.FetchMarkClz`) (`KismetMathLibrary.MakeTransform` (+ _location (0.0 0.0 -10.0)) (struct :`Pitch` -90.0)) "Undefined" "OverrideRootScale" self (`/Game/Blueprints/GlobalFunctions.GetIndexFromXY` X Y) null null))))

(fn `FetchMarkClz`
  (returns (Clz :type "/Game/Blueprints/MarkInst Class Reference"))
  (return "/Game/Blueprints/MarkInst.MarkInst_C"))

(fn `GetWorldPosForXY`)

(fn `SetTargetPoint`
  (params (TargetPoint :type "Vector Structure") (ForceReset :type Boolean))
  (bind _interptomovement (`self.InterpToMovement`))
  (if ForceReset
    (bind _output_get (set `self.Target Point` TargetPoint))
    (`self.K2_SetActorLocation` _output_get)
    (`InterpToMovementComponent.ResetControlPoints` (`self.InterpToMovement`))
    (`PrimitiveComponent.SetCustomPrimitiveDataFloat` (`self.StaticMesh`) 1 (`KismetSystemLibrary.GetGameTimeInSeconds`))
    (elif (> (`KismetMathLibrary.Vector_DistanceSquared` TargetPoint (`self.Target Point`)) 100.0)
      (bind _output_get_2 (set `self.Target Point` TargetPoint))
      (`InterpToMovementComponent.ResetControlPoints` _interptomovement)
      (`InterpToMovementComponent.AddControlPointPosition` _interptomovement (`self.K2_GetActorLocation`) false)
      (`InterpToMovementComponent.AddControlPointPosition` _interptomovement _output_get_2 false)
      (`InterpToMovementComponent.FinaliseControlPoints` _interptomovement)
      (`InterpToMovementComponent.RestartMovement` _interptomovement 1.0))))

(fn `UserConstructionScript`)